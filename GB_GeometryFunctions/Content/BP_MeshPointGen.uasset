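; BP_MeshPointGen is a Blueprint that generates random points within the bounds of its Cone mesh and visualizes them as short-lived debug points.
; BeginPlay or the Init event calls VolumeInterpolator.Init with the cone and its world transform, caching the transformed vertex data and marking it ready.
; Each Tick then runs Gen, which passes that cache to GetRandomPointsInMeshBounds and draws the result.
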(event `self.ReceiveTick`
  (params (DeltaSeconds :type "Float (single-precision)"))
  (`self.Gen`))

(event `self.ReceiveBeginPlay`
  (bind _cone (`self.Cone`))
  (bind _outtransformedvertecies (`VolumeInterpolator.Init` (`self.VolumeInterpolator`) _cone (`SceneComponent.K2_GetComponentToWorld` _cone) true :!label _label))
  (set `self.cached` _outtransformedvertecies)
  (set `self.Cached?` true))

(event `Init`
  (goto _label))

(event `Gen`
  (bind _cone (`self.Cone`))
  (if (`self.Cached?`)
    (bind (_outavgradius _outmaxradius _outtrybox _returnvalue) (`VolumeInterpolator.GetRandomPointsInMeshBounds` (`self.VolumeInterpolator`) _cone (`SceneComponent.K2_GetComponentToWorld` _cone) (`self.cached`) 0))
    (`KismetSystemLibrary.DrawDebugPoint` _returnvalue 10.0 (struct :`R` 0.532172 :`G` 1.0 :`B` 0.365865 :`A` 1.0) 1.0)))

(fn `UserConstructionScript`)