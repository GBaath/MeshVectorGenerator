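; Demo actor that flies a test camera between random points in mesh volumes while aiming it at a moving tracking point.
; On BeginPlay it caches world-space vertex data and bounds for four source and tracking meshes through the VolumeInterpolator.
; Each cycle picks one point per mesh, then Tick applies the curve-driven interpolated location and look-at rotation with debug drawing.
; The interpolator's completion event starts the next randomized cycle, looping continuously.
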(event `self.ReceiveBeginPlay`
  (`self.CalculateAndCacheBounds`)
  (add `VolumeInterpolator.InterpCompletedEvent` (`self.VolumeInterpolator`) (delegate `Redo`)) ; broadcasted when interpolation is completed
  (`self.Redo`))

(event `Redo`
  (`self.debuggen`)
  (`self.StartInterp`))

(event `debuggen`
  (bind (_p1start _p1end _p2start _p2end) (`self.Generate Random Points in Meshes`))
  (set `self.P1Start` _p1start)
  (set `self.P1End` _p1end)
  (set `self.P2Start` _p2start)
  (set `self.P2End` _p2end))

(event `self.ReceiveTick`
  (params (DeltaSeconds :type "Float (single-precision)"))
  (if (`self.DoInterp`)
    (bind (_currentloc _trackingpoint _currentlookatrot _outalpha) (`VolumeInterpolator.TickInterpolate` (`self.VolumeInterpolator`) DeltaSeconds "/GB_GeometryFunctions/DemoInterpolationCurve.DemoInterpolationCurve"))
    (`|ExecutionSequence`
      (:`then_0`
        (`SceneComponent.K2_SetWorldLocationAndRotation` (`self.testCam`) _currentloc _currentlookatrot false false)
        (`KismetSystemLibrary.DrawDebugPoint` _currentloc 10.0 (struct :`G` 1.0 :`B` 0.059102 :`A` 1.0) 0.1)
        (`KismetSystemLibrary.DrawDebugPoint` _trackingpoint 10.0 (struct :`R` 1.0 :`G` 0.522145 :`A` 1.0) 0.1)
        (`KismetSystemLibrary.DrawDebugLine` _currentloc _trackingpoint (struct :`R` 1.0 :`G` 0.257781 :`B` 0.317534 :`A` 1.0) 0.1 1.0)))))

(fn `CalculateAndCacheBounds`
  (locals (Holder :type "Array of Vector Structure") (BHolder :type "Array of Vector Structure"))
  (bind _holder (`local.Holder`))
  (for (_array_element _array_index) (`|MakeArray` (`self.M1Start(Source)`) (`self.M1End(source)`) (`self.M2Start(track)`) (`self.M2End(track)`))
    (bind _outtransformedvertecies (`VolumeInterpolator.Init` (`self.VolumeInterpolator`) _array_element (`SceneComponent.K2_GetComponentToWorld` _array_element) (== _array_index 0)))
    (set `local.Holder` _outtransformedvertecies) ; transformed to world with scale and rot
    (switch `int` _array_index
      (:`0`
        (set `self.VertexDataM1S` _holder))
      (:`1`
        (set `self.VertexDataM1E` _holder))
      (:`2`
        (set `self.VertexDataM2S` _holder))
      (:`3`
        (set `self.VertexDataM2E` _holder))))
  (set `self.Cached bounds` true))

(fn `Generate Random Points in Meshes`
  (returns (P1Start :type "Vector Structure") (P1End :type "Vector Structure") (P2Start :type "Vector Structure") (P2End :type "Vector Structure"))
  (locals (Holder :type "Array of Vector Structure") (OutPoints :type "Array of Vector Structure"))
  (bind _outpoints (`local.OutPoints`))
  (bind _output (`|GetArrayItem` _outpoints 3))
  (bind _output_2 (`|GetArrayItem` _outpoints))
  (bind _output_3 (`|GetArrayItem` _outpoints 1))
  (bind _output_4 (`|GetArrayItem` _outpoints 2))
  (if (`self.Cached bounds`)
    (for (_array_element _array_index) (`|MakeArray` (`self.M1Start(Source)`) (`self.M1End(source)`) (`self.M2Start(track)`) (`self.M2End(track)`))
      (`|ExecutionSequence`
        (:`then_0`
          ;[1 1 1] reassign cached vertexdata
          (switch `int` _array_index
            (:`0`
              (set `local.Holder` (`self.VertexDataM1S`)))
            (:`1`
              (set `local.Holder` (`self.VertexDataM1E`)))
            (:`2`
              (set `local.Holder` (`self.VertexDataM2S`)))
            (:`3`
              (set `local.Holder` (`self.VertexDataM2E`)))))
        (:`then_1`
          (bind (_outavgradius _outmaxradius _outtrybox _returnvalue) (`VolumeInterpolator.GetRandomPointsInMeshBounds` (`self.VolumeInterpolator`) _array_element (`SceneComponent.K2_GetComponentToWorld` _array_element) (`local.Holder`) _array_index))
          (`KismetArrayLibrary.Array_Add` (`local.OutPoints`) _returnvalue))))
    (`|ExecutionSequence`
      (:`then_0`
        ;[1 1 1] debug draw
        (`|ExecutionSequence`
          (:`then_0`
            (`KismetSystemLibrary.DrawDebugPoint` _output_2 10.0 (struct :`R` 1.0 :`G` 0.121708 :`A` 1.0) 1.0))
          (:`then_1`
            (`KismetSystemLibrary.DrawDebugPoint` _output_3 10.0 (struct :`G` 0.151983 :`B` 1.0 :`A` 1.0) 1.0))
          (:`then_2`
            (`KismetSystemLibrary.DrawDebugPoint` _output_4 10.0 (struct :`R` 0.103803 :`G` 1.0 :`B` 0.705769 :`A` 1.0) 1.0))
          (:`then_3`
            (`KismetSystemLibrary.DrawDebugPoint` _output 10.0 (struct :`R` 0.933042 :`G` 0.063542 :`B` 1.0 :`A` 1.0) 1.0))))
      (:`then_1`
        (return _output_2 _output_3 _output_4 _output)))
    (else
      (`KismetSystemLibrary.PrintString` "Generate bounds and chache vertecies before generating"))))

(fn `StartInterp`
  (`VolumeInterpolator.StartInterpolatePoints` (`self.VolumeInterpolator`) false 3.0 (`self.P1Start`) (`self.P1End`) (`self.P2Start`) (`self.P2End`)) ; constant distance = interpvector has const length,\ntime in seconds
  (set `self.DoInterp` true))

(fn `UserConstructionScript`)